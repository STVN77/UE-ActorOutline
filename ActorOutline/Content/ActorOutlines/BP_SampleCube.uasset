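; BP_SampleCube is a sample actor that demonstrates the Outline component's API.
; On BeginPlay, the authority starts a looping half-second timer that sets a random EOutlineColor on the component.
; Outline change and duration-finished events print debug strings.
; Unconnected nodes showcase the component's other functions, such as show/hide, lock/unlock and timed outlines, but never execute.
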(event `self.ReceiveBeginPlay`
  (`/Engine/EditorBlueprintResources/ActorMacros.Switch Has Authority`
    (:`Authority`
      (`KismetSystemLibrary.K2_SetTimerDelegate` (delegate `RandomizeOutline`) 0.5 true))))

(event `RandomizeOutline`
  (`OutlineComponent.SetOutline` (`self.Outline`) (cast `EOutlineColor` (`KismetMathLibrary.Conv_IntToByte` (`KismetMathLibrary.RandomIntegerInRange` 0 5)))))

(event `self.Outline.OnOutlineChanged`
  (`KismetSystemLibrary.PrintString` "Outline Changed"))

(event `self.Outline.OnOutlineDurationFinished`
  (`KismetSystemLibrary.PrintString` "Outline duration finished"))

(fn `UserConstructionScript`)